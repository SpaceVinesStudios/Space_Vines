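; BP_Button is an interactable button that beeps when the player presses Interact while standing near it.
; Overlap events on the Soundtrig trigger set a PlayerClose flag for the player pawn, which gates the Interact input that plays the beep at the trigger's location.
; A timeline meant to flash PointLight1's brightness is present but never runs.
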(event OnComponentBeginOverlap(soundtrig)
  (params (OtherActor :type Actor%20Object%20Reference) (OtherComp :type Primitive%20Component%20Object%20Reference) (OtherBodyIndex :type Integer))
  ;[1 1 1] is player close enoough to press button?
  (if (== OtherActor (Game|Player|GetPlayerPawn 0))
    (Variables|Default|SetplayerClose true)))

(event OnComponentEndOverlap(soundtrig)
  (params (OtherActor :type Actor%20Object%20Reference) (OtherComp :type Primitive%20Component%20Object%20Reference) (OtherBodyIndex :type Integer))
  ;[1 1 1] is player close enoough to press button?
  (if (== OtherActor (Game|Player|GetPlayerPawn 0))
    (Variables|Default|SetplayerClose false)))

(event Input|ActionEvents|InputActionInteract
  ;[1 1 1] if so, BEEP when pressed
  (:Pressed
    (if (Variables|Default|GetplayerClose)
      (Audio|PlaySoundatLocation "/Game/Audio/button_beep.button_beep" (Transformation|GetWorldLocation (Variables|Default|Getsoundtrig)) 0.8))))

(fn ConstructionScript)